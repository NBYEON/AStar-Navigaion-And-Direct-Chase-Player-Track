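; Zombie enemy character that spots, chases, searches for and melee-attacks the player, with a health component driving death.
; A looping timer runs UpdateBrain, using range, view cone and line trace to set Idle, Chase or Search and trigger cooldown-gated attacks.
; Tick applies movement input directly or along waypoints from a custom NavigationZone, turning in place at the last known location.
; Melee damage lands as the montage starts, while movement pauses.
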(event OnDeath(Health)
  (params (HealthComponent :type Survival%20Health%20Component%20Object%20Reference) (KillerActor :type Actor%20Object%20Reference))
  (Variables|Default|SetState "NewEnumerator0")
  (Variables|Default|SetUseDirectMovement false)
  (Utilities|Array|Clear (Variables|Default|GetPathPoint))
  (Actor|Tick|SetActorTickEnabled false)
  (Pawn|Components|CharacterMovement|DisableMovement (Variables|Character|GetCharacterMovement))
  (Components|Animation|PlayAnimation (Variables|Character|GetMesh) "/Game/Characters/Mannequins/Anims/Death/MM_Death_Back_01.MM_Death_Back_01" false)
  (Collision|SetCollisionEnabled (Variables|Collision|GetCapsuleComponent) "NoCollision")
  (Actor|SetLifeSpan 5.0))

(event OnHealthChanged(Health)
  (params (HealthComponent :type Survival%20Health%20Component%20Object%20Reference) (CurrentHealth :type Float%20%28single-precision%29) (MaxHealth :type Float%20%28single-precision%29) (HealthDelta :type Float%20%28single-precision%29) (SourceActor :type Actor%20Object%20Reference))
  (Development|PrintString "damaged"))

(event Custom|StartAttackAnimation
  (if (not (Variables|Default|GetIsAttacking))
    (Variables|Default|SetIsAttacking true)
    (Components|Movement|StopMovementImmediately (Variables|Character|GetCharacterMovement))
    (Animation|PlayAnimMontage "/Game/Characters/Folder/NewFolder/AM_ZombieAtk.AM_ZombieAtk" 1.0 "None")
    (Utilities|FlowControl|Delay 0.8)
    (Variables|Default|SetIsAttacking false)))

(event Custom|BrainTime
  (CallFunction|UpdateBrain))

(event EventBeginPlay
  (Utilities|Time|SetTimerbyEvent (delegate Custom|BrainTime) 0.25 true))

(event Collision|EventActorBeginOverlap
  (params (OtherActor :type Actor%20Object%20Reference)))

(event EventTick
  (params (DeltaSeconds :type Float%20%28single-precision%29))
  (CallFunction|DriveMovement DeltaSeconds))

(fn ConstructionScript)

(fn CanSeePlayer
  (bind _returnvalue (Game|GetPlayerCharacter 0))
  (bind _returnvalue_2 (Transformation|GetActorLocation))
  (bind _returnvalue_3 (Transformation|GetActorLocation _returnvalue))
  (bind _returnvalue_4 (- _returnvalue_3 _returnvalue_2))
  (if (Utilities|IsValid _returnvalue)
    (if (<= (Math|Vector|VectorLength _returnvalue_4) (Variables|Default|GetSightRange))
      (if (>= (Math|Vector|DotProduct (Class|KismetMathLibrary|VectorNormal2D _returnvalue_4 0.0001) (Transformation|GetActorForwardVector)) 0.4)
        (bind (_outhit _returnvalue_5) (Collision|LineTraceByChannel (+ _returnvalue_2 "0.000000,0.000000,60.000000") (+ _returnvalue_3 "0.000000,0.000000,60.000000") "TraceTypeQuery1" false 0 "None"))
        (if _returnvalue_5
          (if (== (.HitActor (Collision|BreakHitResult _outhit)) (Game|GetPlayerCharacter 0))
            (return true)
            (else
              _))))))
  (return false))

(fn UpdateBrain
  (bind _returnvalue (Game|GetPlayerCharacter 0))
  (Variables|Default|SetTimeSinceLastAtk (+ (Variables|Default|GetTimeSinceLastAtk) 0.25))
  (bind _cansee (CallFunction|CanSeePlayer))
  (if _cansee
    (CallFunction|TryMeleeAttack)
    (Variables|Default|SetTargetActor _returnvalue)
    (Variables|Default|SetLastKnownLocation (Transformation|GetActorLocation _returnvalue))
    (Variables|Default|SetTimeSinceSeen 0.0)
    (Variables|Default|SetState "NewEnumerator1")
    (bind _output_get (Variables|Default|SetTimeSinceLastPath (+ (Variables|Default|GetTimeSinceLastPath) 0.25)))
    (if (>= _output_get 0.25)
      (Variables|Default|SetTimeSinceLastPath 0.0)
      (bind _canwalk (Default|CheckDirect (Variables|Default|GetNavigationZone) self (|GetTargetActorLocation)))
      (bind _output_get_2 (Variables|Default|SetUseDirectMovement _canwalk))
      (if _output_get_2
        (Utilities|Array|Clear (Variables|Default|GetPathPoint))
        (else
          (CallFunction|RequestPath (|GetTargetActorLocation_2)))))
    (else
      (Variables|Default|SetTimeSinceSeen (+ (Variables|Default|GetTimeSinceSeen) 0.25))
      (if (Utilities|Enum|Equal(Enum) (Variables|Default|GetState) "NewEnumerator1")
        (Variables|Default|SetState "NewEnumerator2")
        (elif (Utilities|Enum|Equal(Enum) (Variables|Default|GetState) "NewEnumerator2")
          (if (>= (Variables|Default|GetTimeSinceSeen) (Variables|Default|GetSearchDuration))
            (Variables|Default|SetTargetActor 0)
            (Variables|Default|SetState "NewEnumerator0")))))))

(fn DriveMovement
  (params (DeltaSec :type Float%20%28double-precision%29))
  (bind _pathpoint (Variables|Default|GetPathPoint))
  (bind _targetactor (Variables|Default|GetTargetActor))
  (if (Variables|Default|GetIsAttacking)
    (Components|Movement|StopMovementImmediately (Variables|Character|GetCharacterMovement) :!label _label)
    (else
      (switch Utilities|FlowControl|Switch|SwitchonE_ZombieState (Variables|Default|GetState)
        (:NewEnumerator0
          (goto _label))
        (:NewEnumerator1
          (Utilities|IsValid _targetactor
            (:Is%20Valid
              (if (<= (Math|Vector|Distance(Vector) (Transformation|GetActorLocation) (Transformation|GetActorLocation _targetactor)) (Variables|Default|GetStopDistance))
                (goto _label)
                (elif (Variables|Default|GetUseDirectMovement)
                  (Pawn|Input|AddMovementInput (Class|KismetMathLibrary|VectorNormal2D (- (|GetTargetActorLoction) (Transformation|GetActorLocation)) 0.0001) 1.0 false)
                  (else
                    (if (Utilities|Array|IsValidIndex _pathpoint (Variables|Default|GetCurrentPathPoint)) :!label _label_2
                      (if (<= (Math|Vector|VectorLengthXY (- (Utilities|Array|Get(acopy) _pathpoint (Variables|Default|GetCurrentPathPoint)) (Transformation|GetActorLocation))) 1e+01)
                        (Variables|Default|SetCurrentPathPoint (+ (Variables|Default|GetCurrentPathPoint) 1))
                        (else
                          (Pawn|Input|AddMovementInput (Class|KismetMathLibrary|VectorNormal2D (- (Utilities|Array|Get(acopy) _pathpoint (Variables|Default|GetCurrentPathPoint)) (Transformation|GetActorLocation)) 0.0001) 1.0 false)))
                      (else
                        (goto _label)))))))
            (:Is%20Not%20Valid
              (goto _label))))
        (:NewEnumerator2
          (if (<= (Math|Vector|Distance(Vector) (Variables|Default|GetLastKnownLocation) (Transformation|GetActorLocation)) 1e+02)
            (Components|Movement|StopMovementImmediately (Variables|Character|GetCharacterMovement))
            (Transformation|AddActorLocalRotation (Math|Rotator|MakeRotator 0.0 0.0 (* DeltaSec 35.0)) false false)
            (else
              (goto _label_2))))))))

(fn RequestPath
  (params (GoalLoc :type Vector))
  (Utilities|IsValid (Variables|Default|GetNavigationZone)
    (:Is%20Valid
      (bind (_success _waypoints _fail_reason) (Default|RequestPath (Variables|Default|GetNavigationZone) (Transformation|GetActorLocation) GoalLoc))
      (if _success
        (Variables|Default|SetPathPoint _waypoints)
        (Variables|Default|SetCurrentPathPoint 0)
        (else
          (Development|PrintString _fail_reason))))
    (:Is%20Not%20Valid
      (Development|PrintString "no nav zone"))))

(fn TryMeleeAttack
  (bind _targetactor (Variables|Default|GetTargetActor))
  (Utilities|IsValid _targetactor
    (:Is%20Valid
      (if (and (>= (Variables|Default|GetTimeSinceLastAtk) (Variables|Default|GetAtkCooldown)) (<= (Math|Vector|Distance(Vector) (Transformation|GetActorLocation) (Transformation|GetActorLocation (Variables|Default|GetTargetActor))) (Variables|Default|GetMeleeRng)))
        (Variables|Default|SetTimeSinceLastAtk 0.0)
        (CallFunction|StartAttackAnimation)
        (Game|Damage|ApplyDamage _targetactor (Variables|Default|GetMeleeDmg) (Pawn|GetController) self)
        (Variables|Default|SetTimeSinceLastAtk 0.0)))))