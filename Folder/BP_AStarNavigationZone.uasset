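; Navigation zone actor that provides A* pathfinding for zombies through a ZombiePathfinding component.
; On BeginPlay it builds the pathfinding grid.
; RequestPath finds a path between two locations, draws it briefly for debugging and returns success, waypoints and a failure reason.
; CheckDirect reports whether a given character can walk straight to a goal.
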(event EventBeginPlay
  (Class|ZombiePathfindingComponent|BuildGrid (Variables|Default|GetZombiePathfinding)))

(event Collision|EventActorBeginOverlap
  (params (OtherActor :type Actor%20Object%20Reference)))

(event EventTick
  (params (DeltaSeconds :type Float%20%28single-precision%29)))

(fn ConstructionScript)

(fn RequestPath
  (params (StartLoc :type Vector) (GoalLoc :type Vector))
  (bind (_outwaypoints _outfailurereason _returnvalue) (Class|ZombiePathfindingComponent|FindPath (Variables|Default|GetZombiePathfinding) StartLoc GoalLoc))
  (Class|ZombiePathfindingComponent|DrawPath (Variables|Default|GetZombiePathfinding) _outwaypoints 2.0)
  (return _returnvalue _outwaypoints _outfailurereason))

(fn CheckDirect
  (params (MovingChar :type Character%20Object%20Reference) (GoalLoc :type Vector))
  (bind (_outfailurereason _returnvalue) (Class|ZombiePathfindingComponent|CanWalkDirectly (Variables|Default|GetZombiePathfinding) MovingChar GoalLoc))
  (return _returnvalue))